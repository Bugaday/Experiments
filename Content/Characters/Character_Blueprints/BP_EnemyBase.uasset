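; BP_EnemyBase is the base AI enemy character, providing death, gunfire effects, walk/run movement settings and an alert indicator.
; BeginPlay gives the alert widget a dynamic material, whose texture and detection amount are set by helper functions, and applies a mesh constraint profile.
; Death updates the Blackboard's IsDead key and hides the alert.
; Tick rotates the widgets toward the player's camera.
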(event `self.ReceiveBeginPlay`
  ;[1 1 1] Begin Play
  (`|ExecutionSequence`
    (:`then_0`
      (bind _asalert_widget (cast `/Game/UI/Widgets/AlertWidget` (`WidgetComponent.GetUserWidgetObject` (`self.Alert`))))
      (bind _returnvalue (`KismetMaterialLibrary.CreateDynamicMaterialInstance` "/Game/UI/Widgets/mat_AlertStatus_Inst.mat_AlertStatus_Inst"))
      (bind _output_get (set `/Game/UI/Widgets/AlertWidget.DynamicMat` _returnvalue _asalert_widget))
      (`Image.SetBrushFromMaterial` (`/Game/UI/Widgets/AlertWidget.MainImage` _asalert_widget) _output_get))
    (:`then_1`
      (`SkeletalMeshComponent.SetConstraintProfileForAll` (`self.Mesh`) (`self.ConstraintsName`) true))))

(event `self.ReceiveTick`
  (params (DeltaSeconds :type "Float (single-precision)"))
  ;[1 1 1] Tick
  (`self.MakeWidgetFaceCamera`))

(fn `Attack`
  (set `self.IsAiming` true)
  (`GameplayStatics.PlaySound2D` "/Game/Blueprints/Items/Weapons/WeaponAudio/MP5-Burst-Stereo_Cue.MP5-Burst-Stereo_Cue" 1.0 1.0 0.0 null null)
  (`GameplayStatics.SpawnEmitterAttached` "/Game/Blueprints/Items/Weapons/WeaponEffects/Custom_FX_Gunshot_Repeating.Custom_FX_Gunshot_Repeating" (`self.FirePoint`)))

(fn `Death`
  (set `self.IsDead` true)
  (`BlackboardComponent.SetValueAsBool` (`AIController.Blackboard` (`AIBlueprintHelperLibrary.GetAIController` self)) "IsDead" true)
  (set `self.IsStaggered` false)
  (`SceneComponent.SetVisibility` (`self.Alert`) false false))

(fn `GetMyBlackBoard`
  (returns (Blackboard :type "BlackboardComponent Object Reference"))
  (return (`AIController.Blackboard` (`AIBlueprintHelperLibrary.GetAIController` self))))

(fn `MakeWidgetFaceCamera`
  (bind _ascharacter_main_character (cast `/Game/Characters/Character_Blueprints/Character_MainCharacter` (`Controller.K2_GetPawn` (`GameplayStatics.GetPlayerController` 0))))
  (`SceneComponent.K2_SetWorldRotation` (`self.Widgets`) (`KismetMathLibrary.FindLookAtRotation` (`SceneComponent.K2_GetComponentLocation` (`self.Widgets`)) (`SceneComponent.K2_GetComponentLocation` (`/Game/Characters/Character_Blueprints/Character_MainCharacter.PlayerCamera` _ascharacter_main_character))) false false))

(fn `SetAlertTextureImage`
  (params (Value :type "Texture Object Reference"))
  (bind _asalert_widget (cast `/Game/UI/Widgets/AlertWidget` (`WidgetComponent.GetUserWidgetObject` (`self.Alert`))))
  (`MaterialInstanceDynamic.SetTextureParameterValue` (`/Game/UI/Widgets/AlertWidget.DynamicMat` _asalert_widget) "Texture" Value))

(fn `SetInvestigationWidget`
  (params (`Investigation Time` :type "Float (double-precision)"))
  (bind _asalert_widget (cast `/Game/UI/Widgets/AlertWidget` (`WidgetComponent.GetUserWidgetObject` (`self.Alert`))))
  (`MaterialInstanceDynamic.SetScalarParameterValue` (`/Game/UI/Widgets/AlertWidget.DynamicMat` _asalert_widget) "DetectedAmount" `Investigation Time`))

(fn `SetRunMovementAndRotation`
  (bind _charactermovement (`self.CharacterMovement`))
  (set `CharacterMovementComponent.MaxWalkSpeed` (`self.RunSpeed`) _charactermovement)
  (set `CharacterMovementComponent.RotationRate` (`KismetMathLibrary.MakeRotator` 0.0 0.0 (`self.RunRotationRate`)) _charactermovement))

(fn `SetWalkMovementAndRotation`
  (bind _charactermovement (`self.CharacterMovement`))
  (set `CharacterMovementComponent.MaxWalkSpeed` (`self.WalkSpeed`) _charactermovement)
  (set `CharacterMovementComponent.RotationRate` (`KismetMathLibrary.MakeRotator` 0.0 0.0 (`self.WalkRotationRate`)) _charactermovement))

(fn `UserConstructionScript`)