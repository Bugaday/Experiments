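; Player controller for a sniper game that adds the base HUD widget, caches the sniper pawn and runs one test shot on BeginPlay.
; Snipe approximates a ballistic arc with chained line-trace segments, stepping along the pawn's forward vector by muzzle velocity with gravity drop growing each step.
; It only visualizes the path with rainbow debug lines and endpoint spheres; trace hits are never used.
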(event `self.ReceiveBeginPlay`
  (`|ExecutionSequence`
    (:`then_0`
      (bind _returnvalue (`|CreateWidget` "/Game/Sniper/UMG_SniperBase.UMG_SniperBase_C"))
      (bind _output_get (set `self.UI_Base` _returnvalue))
      (`UserWidget.AddToViewport` _returnvalue 0)
      (`UserWidget.AddToViewport` _output_get 0))
    (:`then_1`
      (bind _asbp_sniper_player (cast `/Game/Sniper/BP_SniperPlayer` (`self.K2_GetPawn`)))
      (set `self.SniperPlayer` _asbp_sniper_player))
    (:`then_2`
      (`self.Snipe`))))

(event `Snipe`
  (bind _lastendpoint (`self.LastEndPoint`))
  (bind _sniperplayer (`self.SniperPlayer`))
  (set `self.LastStartPoint` (`self.K2_GetActorLocation` (`self.SniperPlayer`)))
  (set `self.LastEndPoint` (+ (`self.K2_GetActorLocation` _sniperplayer) (* (`self.GetActorForwardVector` _sniperplayer) (`self.MuzzleVelocity`))))
  (for _index (range 51)
    (set `self.RayIndex` _index)
    (`KismetSystemLibrary.LineTraceSingle` :`Start` (`self.LastStartPoint`) :`End` (`self.LastEndPoint`) :`TraceChannel` "TraceTypeQuery1" :`DrawDebugType` "ForDuration" :`TraceColor` (`KismetMathLibrary.HSVToRGB` (* (`KismetMathLibrary.Conv_IntToDouble` _index) (/ 360.0 50.0)) 1.0 1.0) :`DrawTime` 20.0)
    (`KismetSystemLibrary.DrawDebugSphere` (`self.LastEndPoint`) 10.0 12 (struct :`R` 0.933621 :`G` 0.20975 :`B` 1.0 :`A` 1.0) 20.0 1.0)
    (set `self.LastStartPoint` _lastendpoint)
    (set `self.LastEndPoint` (- (+ _lastendpoint (* (`self.GetActorForwardVector` (`self.SniperPlayer`)) (`self.MuzzleVelocity`))) (`KismetMathLibrary.MakeVector` 0.0 0.0 (* (`self.Gravity`) (`KismetMathLibrary.Conv_IntToDouble` (`self.RayIndex`))))))))

(fn `UserConstructionScript`)