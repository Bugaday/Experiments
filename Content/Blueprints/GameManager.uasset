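; GameManager actor that runs a mark-and-execute mechanic, holding the list of marked enemies through AddTarget and RemoveTarget.
; ExecuteTargets disables player input, puts the character in an aiming pose with camera boom detached from control rotation, then starts a looping Execute timer.
; Each tick turns control yaw toward the first target, kills and unmarks it, clearing the timer once none remain.
; Input, camera and aim restore after a fixed delay, independent of remaining targets.
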(event `ExecuteTargets`
  (if (> (`KismetArrayLibrary.Array_Length` (`self.MarkedTargets`)) 0)
    (`self.DisableInput` (`GameplayStatics.GetPlayerPawn` 0) (`GameplayStatics.GetPlayerController` 0))
    (bind _ascharacter_mannequin (cast `/Game/Characters/Character_Blueprints/Character_MainCharacter` (`GameplayStatics.GetPlayerPawn` 0)))
    (set `SpringArmComponent.bUsePawnControlRotation` false (`/Game/Characters/Character_Blueprints/Character_MainCharacter.CameraBoom` _ascharacter_mannequin))
    (set `/Game/Characters/Character_Blueprints/Character_MainCharacter.IsAiming` true _ascharacter_mannequin)
    (`KismetSystemLibrary.Delay` 0.5)
    (`KismetSystemLibrary.K2_SetTimer` null "Execute" 1.0 true)
    (`KismetSystemLibrary.Delay` 1.0)
    (bind _ascharacter_mannequin_2 (cast `/Game/Characters/Character_Blueprints/Character_MainCharacter` (`GameplayStatics.GetPlayerPawn` 0)))
    (set `/Game/Characters/Character_Blueprints/Character_MainCharacter.IsAiming` false _ascharacter_mannequin_2)
    (set `SpringArmComponent.bUsePawnControlRotation` true (`/Game/Characters/Character_Blueprints/Character_MainCharacter.CameraBoom` _ascharacter_mannequin_2))
    (`self.EnableInput` (`GameplayStatics.GetPlayerPawn` 0) (`GameplayStatics.GetPlayerController` 0))))

(fn `AddTarget`
  (params (EnemyToAdd :type "/Game/Characters/Character_Blueprints/Character_AI Object Reference"))
  (`KismetArrayLibrary.Array_Add` (`self.MarkedTargets`) EnemyToAdd))

(fn `Execute`
  (locals (ExecutedEnemy :type "/Game/Characters/Character_Blueprints/Character_AI Object Reference"))
  (bind _returnvalue (`GameplayStatics.GetPlayerController` 0))
  (bind _executedenemy (`local.ExecutedEnemy`))
  (bind (_returnvalue_roll _returnvalue_pitch _returnvalue_yaw) (`KismetMathLibrary.BreakRotator` (`KismetMathLibrary.FindLookAtRotation` (`self.K2_GetActorLocation` _returnvalue) (`self.K2_GetActorLocation` (`local.ExecutedEnemy`)))))
  (bind _output_get (set `local.ExecutedEnemy` (`|GetArrayItem` (`self.MarkedTargets`))))
  (`Controller.SetControlRotation` _returnvalue (`KismetMathLibrary.MakeRotator` 0.0 0.0 _returnvalue_yaw))
  (`/Game/Characters/Character_Blueprints/Character_AI.Death` _output_get)
  (set `/Game/Characters/Character_Blueprints/Character_AI.IsMarked` false _executedenemy)
  (`SceneComponent.SetVisibility` (`/Game/Characters/Character_Blueprints/Character_AI.Marker` _executedenemy) false false)
  (`KismetArrayLibrary.Array_RemoveItem` (`self.MarkedTargets`) (`local.ExecutedEnemy`))
  (if (< (`KismetArrayLibrary.Array_Length` (`self.MarkedTargets`)) 1)
    (`KismetSystemLibrary.K2_ClearTimer` null "Execute")))

(fn `RemoveTarget`
  (params (EnemyToRemove :type "/Game/Characters/Character_Blueprints/Character_AI Object Reference"))
  (`KismetArrayLibrary.Array_RemoveItem` (`self.MarkedTargets`) EnemyToRemove))

(fn `UserConstructionScript`)